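; BP_AIRandom is an AI pawn, apparently a clown, that wanders the NavMesh and chases the player on sight.
; MoveRandom loops AI moves to random reachable points nearby, drawing green or red debug points for success or failure.
; Pawn sensing triggers a one-time sound and timed dialogue bubble widget, then chases a visible, reachable BP_TopDownHero.
; It resumes wandering when the hero is hiding, unreachable, or the chase move ends.
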(event `self.ReceiveBeginPlay`
  (`self.MoveRandom`))

(event `MoveRandom`
  ; Move Randomly in the NavMesh
  (bind _randomlocation (`NavigationSystemV1.K2_GetRandomLocationInNavigableRadius` (`self.K2_GetActorLocation`) 500.0 null null))
  (`|AIMoveTo` self _randomlocation null
    (:`OnSuccess`
      (`KismetSystemLibrary.DrawDebugPoint` _randomlocation 2.0 (struct :`G` 0.90625 :`B` 0.053749 :`A` 1.0) 5.0))
    (:`OnFail`
      (`KismetSystemLibrary.DrawDebugPoint` _randomlocation 2.0 (struct :`R` 0.802083 :`G` 0.009912 :`A` 1.0) 5.0)))
  (`self.MoveRandom`))

(event `self.PawnSensing.OnSeePawn`
  (params (Pawn :type "Pawn Object Reference"))
  (if (not (`self.HasShownBubbleDetectClown`))
    (`GameplayStatics.PlaySound2D` "/Game/SoundDesign/SOUNDS/Hoho-clown_Cue.Hoho-clown_Cue" 1.0 1.0 0.0 null null)
    (`self.ShowBubbleAI` 0 3.0)
    (set `self.HasShownBubbleDetectClown` true))
  (bind _asbp_top_down_hero (cast `/Game/Blueprints/BP_TopDownHero` Pawn))
  (if (`/Game/Blueprints/BP_TopDownHero.isHiding` _asbp_top_down_hero)
    (`self.MoveRandom`)
    (else
      (bind _returnvalue (`NavigationSystemV1.FindPathToActorSynchronously` (`self.K2_GetActorLocation`) Pawn 50.0 null null))
      (if (`NavigationPath.IsValid` _returnvalue)
        (`|AIMoveTo` self (0.0 0.0 0.0) Pawn
          (:`OnSuccess`
            _)
          (:`OnFail`
            _))
        (`self.MoveRandom`)
        (else
          (`self.MoveRandom`))))))

(event `self.ShowBubbleAI`
  (params (NumberOfBubble :type Integer) (DurationBubble :type "Float (double-precision)"))
  (bind _widget (`self.Widget`))
  ; Show Dialogue Bubble over Player's head when enter trigger in level
  (bind _aswd_bubble_clown (cast `/Game/UI/HUD-SpeechBubbles/WD_Bubble_CLOWN` (`WidgetComponent.GetUserWidgetObject` _widget)))
  (`/Game/UI/HUD-SpeechBubbles/WD_Bubble_CLOWN.SetBubble` _aswd_bubble_clown NumberOfBubble)
  (`SceneComponent.SetVisibility` _widget true false)
  (if (== NumberOfBubble 1)
    (`GameplayStatics.PlaySound2D` "/Game/SoundDesign/SOUNDS/Cri-homme_Cue.Cri-homme_Cue" 1.0 1.0 0.0 null null))
  (`KismetSystemLibrary.Delay` DurationBubble)
  (`SceneComponent.SetVisibility` _widget false false))

(fn `UserConstructionScript`
  (`parent.UserConstructionScript`))