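; Switchable spotlight hazard that blocks AI navigation and removes BP_AI actors caught in its cone when powered.
; PowerOn lights the spot, nulls its nav area, shows bubbles on overlapping AI and the player hero, and destroys AI after a Delay inside the loop, which does not wait per actor.
; PowerOff turns the light off and restores default navigation.
; The construction script applies the configurable cone angle and detection-cone scale.
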(event `PowerOn`
  (`LightComponent.SetIntensity` (`self.SpotLight`) 1000000.0)
  (`NavModifierComponent.SetAreaClass` (`self.NavModifier`) "/Script/NavigationSystem.NavArea_Null")
  (for _array_element (`PrimitiveComponent.GetOverlappingActors` (`self.Cone`) "/Game/Blueprints/BP_AI.BP_AI_C")
    ; How to know if it's doll or Clown?
    (bind _asbp_ai (cast `/Game/Blueprints/BP_AI` _array_element))
    (`/Game/Blueprints/BP_AI.ShowBubbleDoll` _asbp_ai 1 1.5)
    (`KismetSystemLibrary.Delay` 1.5)
    (`self.K2_DestroyActor` _array_element))
  (bind _asbp_top_down_hero (cast `/Game/Blueprints/BP_TopDownHero` (`GameplayStatics.GetPlayerCharacter` 0)))
  (`/Game/Blueprints/BP_TopDownHero.ShowBubble` _asbp_top_down_hero 4 2.0))

(event `PowerOff`
  (`LightComponent.SetIntensity` (`self.SpotLight`) 0.0)
  (`NavModifierComponent.SetAreaClass` (`self.NavModifier`) "/Script/NavigationSystem.NavArea_Default"))

(fn `UserConstructionScript`
  (`SpotLightComponent.SetOuterConeAngle` (`self.SpotLight`) (`self.OuterConeAngle`))
  (`SceneComponent.SetWorldScale3D` (`self.Cone`) (`self.ScaleCone`)))