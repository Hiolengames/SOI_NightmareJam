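; Enemy AI pawn, with a doll variant, that patrols looping waypoints and threatens the top-down hero.
; When IsDoll is set, PawnSensing triggers a chase of the visible hero, with a one-time sound and widget bubble, then returns to patrol.
; Overlapping an unhidden hero deals damage and destroys the AI if CanDamage allows.
; Exposes bubble and PaperZD fear-animation events; a damage-cooldown chain is left unwired.
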(event `self.ReceiveBeginPlay`
  (`KismetSystemLibrary.Delay` 2.0)
  (`self.FollowWaypoints`))

(event `FollowWaypoints`
  ; Pathing between different waypoints
  (`|AIMoveTo` self (0.0 0.0 0.0) (`|GetArrayItem` (`self.waypoints`) (`self.currentWaypoint`))
    (:`OnSuccess`
      (`/Engine/EditorBlueprintResources/StandardMacros.IncrementInt` (`self.currentWaypoint`)
        (:`  `
          (if (>= (`self.currentWaypoint`) (`KismetArrayLibrary.Array_Length` (`self.waypoints`)))
            (set `self.currentWaypoint` 0))
          (`KismetSystemLibrary.Delay` 1.0)
          (`self.FollowWaypoints`))))
    (:`OnFail`
      (`self.FollowWaypoints`))))

(event `self.PawnSensing.OnSeePawn`
  (params (Pawn :type "Pawn Object Reference"))
  ; Detect player then chase him
  (if (`self.isDoll`)
    (bind _asbp_top_down_hero (cast `/Game/Blueprints/BP_TopDownHero` Pawn))
    (if (`/Game/Blueprints/BP_TopDownHero.isHiding` _asbp_top_down_hero)
      (`self.FollowWaypoints`)
      (else
        (if (not (`self.HasShownBubbleDetect`))
          (`self.PlayOneTimeSoundAndBubble`))
        (`|AIMoveTo` self (0.0 0.0 0.0) Pawn
          (:`OnSuccess`
            _)
          (:`OnFail`
            _))
        (`KismetSystemLibrary.Delay` 1.0)
        (`self.FollowWaypoints`)))))

(event `PlayOneTimeSoundAndBubble`
  ; Detect player then chase him
  (`GameplayStatics.PlaySound2D` "/Game/SoundDesign/SOUNDS/Rire-enfant2_Cue.Rire-enfant2_Cue" 1.0 1.0 0.0 null null)
  (`self.ShowBubbleAI` 0 3.5)
  (set `self.HasShownBubbleDetect` true))

(event `self.PlayerOverlapTrigger.OnComponentBeginOverlap`
  (params (OverlappedComponent :type "PrimitiveComponent Object Reference") (OtherActor :type "Actor Object Reference") (OtherComp :type "PrimitiveComponent Object Reference") (OtherBodyIndex :type Integer) (bFromSweep :type Boolean) (SweepResult :type "HitResult Structure (by ref)"))
  ; Attack player on Overlap then destroy itself
  (bind _asbp_top_down_hero (cast `/Game/Blueprints/BP_TopDownHero` OtherActor))
  (if (and (not (`/Game/Blueprints/BP_TopDownHero.isHiding` _asbp_top_down_hero)) (`self.CanDamage`))
    (`/Game/Blueprints/BP_TopDownHero.TakeDamage` _asbp_top_down_hero)
    (`self.K2_DestroyActor`)))

(event `ShowBubbleAI`
  (params (NumberOfBubble :type Integer) (DurationBubble :type "Float (double-precision)" :default 3.0))
  (bind _widget (`self.Widget`))
  ; Show Bubble when AI is hit by Light
  (bind _aswd_bubble_doll (cast `/Game/UI/HUD-SpeechBubbles/WD_Bubble_DOLL` (`WidgetComponent.GetUserWidgetObject` _widget)))
  (`/Game/UI/HUD-SpeechBubbles/WD_Bubble_DOLL.SetBubble` _aswd_bubble_doll NumberOfBubble)
  (`SceneComponent.SetVisibility` _widget true false)
  (if (== NumberOfBubble 1)
    (`GameplayStatics.PlaySound2D` "/Game/SoundDesign/SOUNDS/Cri-fille_Cue.Cri-fille_Cue" 1.0 1.0 0.0 null null))
  (`KismetSystemLibrary.Delay` DurationBubble)
  (`SceneComponent.SetVisibility` _widget false false))

(event `ChangeToFearAnim`
  (`PaperZDAnimInstance.JumpToNode` (`PaperZDAnimationComponent.AnimInstance` (`self.PaperZDAnimation`)) "Death" "None"))

(fn `UserConstructionScript`)