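; A table hiding spot for the top-down hero.
; Overlapping the BoxLeft trigger sets the hero's IsHiding flag, hides its sprite and turns off pawn sensing updates on every BP_AI actor in the level.
; Leaving the box reverses all three, using a fresh GetAllActorsOfClass lookup each time.
; The Interact event has no logic.
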(event `/Game/Blueprints/InteractInterface.Interact`)

(event `self.BoxLeft.OnComponentBeginOverlap`
  (params (OverlappedComponent :type "PrimitiveComponent Object Reference") (OtherActor :type "Actor Object Reference") (OtherComp :type "PrimitiveComponent Object Reference") (OtherBodyIndex :type Integer) (bFromSweep :type Boolean) (SweepResult :type "HitResult Structure (by ref)"))
  (bind _asbp_top_down_hero (cast `/Game/Blueprints/BP_TopDownHero` OtherActor))
  (set `/Game/Blueprints/BP_TopDownHero.isHiding` true _asbp_top_down_hero)
  (`SceneComponent.SetVisibility` (`PaperCharacter.Sprite` _asbp_top_down_hero) false false)
  (bind _outactors (`GameplayStatics.GetAllActorsOfClass` "/Game/Blueprints/BP_AI.BP_AI_C"))
  (for _array_element _outactors
    (`PawnSensingComponent.SetSensingUpdatesEnabled` (`/Game/Blueprints/BP_AI.PawnSensing` _array_element) false)))

(event `self.BoxLeft.OnComponentEndOverlap`
  (params (OverlappedComponent :type "PrimitiveComponent Object Reference") (OtherActor :type "Actor Object Reference") (OtherComp :type "PrimitiveComponent Object Reference") (OtherBodyIndex :type Integer))
  (bind _asbp_top_down_hero (cast `/Game/Blueprints/BP_TopDownHero` OtherActor))
  (set `/Game/Blueprints/BP_TopDownHero.isHiding` false _asbp_top_down_hero)
  (`SceneComponent.SetVisibility` (`PaperCharacter.Sprite` _asbp_top_down_hero) true false)
  (bind _outactors (`GameplayStatics.GetAllActorsOfClass` "/Game/Blueprints/BP_AI.BP_AI_C"))
  (for _array_element _outactors
    (`PawnSensingComponent.SetSensingUpdatesEnabled` (`/Game/Blueprints/BP_AI.PawnSensing` _array_element) true)))

(fn `UserConstructionScript`)