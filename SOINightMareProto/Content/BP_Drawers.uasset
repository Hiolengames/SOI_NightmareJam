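; BP_Drawers is an interactable drawer the player hides in to avoid AI detection.
; Each Interact alternates through a FlipFlop between entering and leaving, teleporting the hero between TPHide and TPNotHide and toggling movement and IsHiding.
; Hiding disables PawnSensing on every BP_AI and leaving restores it.
; On entry, the teleport and speech bubble run inside the AI loop, so they repeat per AI.
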(event `/Game/Blueprints/InteractInterface.Interact`
  (bind _returnvalue (`GameplayStatics.GetPlayerCharacter` 0))
  (bind _returnvalue_2 (`GameplayStatics.GetPlayerCharacter` 0))
  (bind _returnvalue_3 (`GameplayStatics.GetPlayerCharacter` 0))
  ; Player interaction with the drawer (get tped in it)
  (`/Engine/EditorBlueprintResources/StandardMacros.FlipFlop`
    (:`A`
      ;; Player is tped in the drawer
      (`CharacterMovementComponent.SetMovementMode` (`Character.CharacterMovement` _returnvalue_2) "MOVE_None" 0)
      (bind _asbp_top_down_hero (cast `/Game/Blueprints/BP_TopDownHero` _returnvalue_2))
      (set `/Game/Blueprints/BP_TopDownHero.isHiding` true _asbp_top_down_hero)
      (bind _outactors (`GameplayStatics.GetAllActorsOfClass` "/Game/Blueprints/BP_AI.BP_AI_C"))
      (for _array_element _outactors
        (`PawnSensingComponent.SetSensingUpdatesEnabled` (`/Game/Blueprints/BP_AI.PawnSensing` _array_element) false)
        (`self.K2_TeleportTo` :`self` _asbp_top_down_hero :`DestLocation` (`SceneComponent.K2_GetComponentLocation` (`self.TPHide`)))
        (`CharacterMovementComponent.SetMovementMode` (`Character.CharacterMovement` _returnvalue) "MOVE_None" 0)
        (bind _asbp_top_down_hero_2 (cast `/Game/Blueprints/BP_TopDownHero` _returnvalue))
        (`/Game/Blueprints/BP_TopDownHero.ShowBubble` _asbp_top_down_hero_2 3 4.0)))
    (:`B`
      ;; Player is tped out of the drawer
      (`CharacterMovementComponent.SetMovementMode` (`Character.CharacterMovement` _returnvalue_3) "MOVE_Walking" 0)
      (bind _asbp_top_down_hero_3 (cast `/Game/Blueprints/BP_TopDownHero` _returnvalue_3))
      (`self.K2_TeleportTo` :`self` _asbp_top_down_hero_3 :`DestLocation` (`SceneComponent.K2_GetComponentLocation` (`self.TPNotHide`)))
      (set `/Game/Blueprints/BP_TopDownHero.isHiding` false _asbp_top_down_hero_3)
      (bind _outactors_2 (`GameplayStatics.GetAllActorsOfClass` "/Game/Blueprints/BP_AI.BP_AI_C"))
      (for _array_element_2 _outactors_2
        (`PawnSensingComponent.SetSensingUpdatesEnabled` (`/Game/Blueprints/BP_AI.PawnSensing` _array_element_2) true)))))

(fn `UserConstructionScript`)