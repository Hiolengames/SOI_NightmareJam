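; BP_Locker is an interactable locker that moves the player character in and out by teleporting it.
; Interact alternates through a FlipFlop: entering disables movement and teleports BP_TopDownHero to the Cube component, exiting restores walking and teleports it to the Scene component.
; Capsule collision is switched off only for the duration of the teleport into the locker, then re-enabled immediately.
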(event `/Game/Blueprints/InteractInterface.Interact`
  (bind _returnvalue (`GameplayStatics.GetPlayerCharacter` 0))
  (bind _returnvalue_2 (`GameplayStatics.GetPlayerCharacter` 0))
  (bind _capsulecomponent (`Character.CapsuleComponent` _returnvalue))
  ; Player interaction with the locker (get tped in it)
  (`/Engine/EditorBlueprintResources/StandardMacros.FlipFlop`
    (:`A`
      ;; Player is tped in the locker
      (`CharacterMovementComponent.DisableMovement` (`Character.CharacterMovement` _returnvalue))
      (bind _asbp_top_down_hero (cast `/Game/Blueprints/BP_TopDownHero` _returnvalue))
      (`PrimitiveComponent.SetCollisionEnabled` _capsulecomponent "NoCollision")
      (`self.K2_TeleportTo` :`self` _asbp_top_down_hero :`DestLocation` (`SceneComponent.K2_GetComponentLocation` (`self.Cube`)))
      (`PrimitiveComponent.SetCollisionEnabled` _capsulecomponent "QueryAndPhysics")
      (`KismetSystemLibrary.PrintText` "TP in locker"))
    (:`B`
      ;; Player is tped out of the locker
      (`CharacterMovementComponent.SetMovementMode` (`Character.CharacterMovement` _returnvalue_2) "MOVE_Walking" 0)
      (bind _asbp_top_down_hero_2 (cast `/Game/Blueprints/BP_TopDownHero` _returnvalue_2))
      (`self.K2_TeleportTo` :`self` _asbp_top_down_hero_2 :`DestLocation` (`SceneComponent.K2_GetComponentLocation` (`self.Scene`))))))

(fn `UserConstructionScript`)